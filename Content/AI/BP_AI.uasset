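; BP_AI is an armed enemy that shoots its AI controller's focus actor using line-traced point damage with muzzle and impact effects.
; ApplyDamage drains armor before health, and a successful shot writes normalized health to the Blackboard.
; A sphere overlap shows the health bar widget only while the player is near.
; Tick polls for zero health, then rewards XP and currency, reports the quest kill and destroys the actor.
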(event `self.ReceiveBeginPlay`
  (set `self.health` (`self.maxhealth`))
  (`self.UpdateHealthBar`))

(event `self.ReceiveTick`
  (params (DeltaSeconds :type "Float (single-precision)"))
  (if (== (`self.health`) 0.0)
    (bind _asbp_first_person_character (cast `/Game/FirstPerson/Blueprints/BP_FirstPersonCharacter` (`GameplayStatics.GetPlayerCharacter` 0)))
    (`/Game/FirstPerson/Blueprints/BP_FirstPersonCharacter.Gain XP` _asbp_first_person_character 500.0)
    (`/Game/InventorySystem/InventoryComponent.Update Currency` (`self.PlayerInv`) 50)
    (bind _asbp_first_person_character_2 (cast `/Game/FirstPerson/Blueprints/BP_FirstPersonCharacter` (`GameplayStatics.GetPlayerCharacter` 0)))
    (`/Game/FirstPerson/Blueprints/BP_FirstPersonCharacter.Quest Enemy Killed` _asbp_first_person_character_2)
    (`self.K2_DestroyActor`)))

(event `StartShooting`
  (bind _returnvalue (`AIController.GetFocusActor` (`AIBlueprintHelperLibrary.GetAIController` self)))
  (`/Engine/EditorBlueprintResources/StandardMacros.IsValid` _returnvalue
    (:`Is Valid`
      (bind (_outhit _returnvalue_2) (`KismetSystemLibrary.LineTraceSingle` (`SceneComponent.K2_GetComponentLocation` (`self.Weapon`)) (`self.K2_GetActorLocation` _returnvalue) "TraceTypeQuery2"))
      (`GameplayStatics.SpawnEmitterAttached` "/Game/MilitaryWeapSilver/FX/P_Pistol_MuzzleFlash_01.P_Pistol_MuzzleFlash_01" (`self.Weapon`) "MuzzleFlash")
      (if _returnvalue_2
        (bind (_bblockinghit _binitialoverlap _time _distance _location _impactpoint _normal _impactnormal _physmat _hitactor) (`GameplayStatics.BreakHitResult` _outhit))
        (`GameplayStatics.SpawnEmitterAtLocation` "/Game/MilitaryWeapSilver/FX/P_Impact_Metal_Small_01.P_Impact_Metal_Small_01" _location (`KismetMathLibrary.MakeRotFromX` _impactnormal))
        (`GameplayStatics.ApplyPointDamage` _hitactor (`self.Base Damage`) _impactnormal _outhit null self)
        (`self.UpdateBBHealth`)))))

(event `self.Sphere.OnComponentBeginOverlap`
  (params (OverlappedComponent :type "PrimitiveComponent Object Reference") (OtherActor :type "Actor Object Reference") (OtherComp :type "PrimitiveComponent Object Reference") (OtherBodyIndex :type Integer) (bFromSweep :type Boolean) (SweepResult :type "HitResult Structure (by ref)"))
  (cast `/Game/FirstPerson/Blueprints/BP_FirstPersonCharacter` OtherActor)
  (`SceneComponent.SetVisibility` (`self.HeatlhBar`) true false))

(event `self.Sphere.OnComponentEndOverlap`
  (params (OverlappedComponent :type "PrimitiveComponent Object Reference") (OtherActor :type "Actor Object Reference") (OtherComp :type "PrimitiveComponent Object Reference") (OtherBodyIndex :type Integer))
  (cast `/Game/FirstPerson/Blueprints/BP_FirstPersonCharacter` OtherActor)
  (`SceneComponent.SetVisibility` (`self.HeatlhBar`) false false))

(fn `Apply Damage`
  (params (Damage :type "Float (double-precision)"))
  (returns (Health :type "Float (double-precision)"))
  (if (> (`self.armor`) 0.0)
    (set `self.armor` (`KismetMathLibrary.FClamp` (- (`self.armor`) Damage) 0.0 (`self.maxArmor`)))
    (else
      (bind _output_get (set `self.health` (`KismetMathLibrary.FClamp` (- (`self.health`) Damage) 0.0 (`self.maxhealth`))))))
  (return _output_get))

(fn `SetArmor`
  (set `self.armor` (`self.maxArmor`)))

(fn `UpdateBBHealth`
  (`BlackboardComponent.SetValueAsFloat` (`AIBlueprintHelperLibrary.GetBlackboard` null) "Health" (`KismetMathLibrary.NormalizeToRange` (`self.health`) 0.0 (`self.maxhealth`))))

(fn `UpdateHealthBar`
  (bind _asenemy_hpbar (cast `/Game/UI/EnemyHPBar` (`WidgetComponent.GetUserWidgetObject` (`self.HeatlhBar`))))
  (set `/Game/UI/EnemyHPBar.Heatlh` (`self.health`) _asenemy_hpbar)
  (return))

(fn `UserConstructionScript`)