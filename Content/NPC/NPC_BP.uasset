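; NPC Blueprint for a quest giver whose Talk event steps through one of three dialogue arrays, chosen by whether Quest1 is unstarted, in progress or complete.
; Each call advances a shared TalkIndex, shows that line in a Dialogue_WB widget with a sound, and resets past the array's end.
; Reaching the third start line sets Quest1Start and the "Collect the Macguffin." objective, without resetting the index.
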(event `/Game/NPC/Dialogue_BPI.Talk`
  (if (`self.Quest1Start`)
    (if (`self.Quest1Complete`)
      (`Widget.RemoveFromParent` (`self.UI`))
      (`/Engine/EditorBlueprintResources/StandardMacros.IncrementInt` (`self.TalkIndex`)
        (:`  `
          (if (< (`self.TalkIndex`) (`KismetArrayLibrary.Array_Length` (`self.DialogueQuest1Complete`)))
            (bind _returnvalue (`|CreateWidget` "/Game/NPC/Dialogue_WB.Dialogue_WB_C" (`GameplayStatics.GetPlayerController` 0)))
            (bind _output_get (set `self.UI` _returnvalue))
            (`UserWidget.AddToViewport` _output_get 0)
            ;[1 1 1] Play Dialogue if Quest is Complete
            (`TextBlock.SetText` (`/Game/NPC/Dialogue_WB.TalkText` (`self.UI`)) (`KismetTextLibrary.Conv_StringToText` (`|GetArrayItem` (`self.DialogueQuest1Complete`) (`self.TalkIndex`))))
            (`GameplayStatics.PlaySound2D` "/Game/MilitaryWeapSilver/Sound/Knife/Wavs/Knife_ImpactSurface03.Knife_ImpactSurface03" 1.0 1.0 0.0 null null)
            (else
              (set `self.TalkIndex` -1)
              (`Widget.RemoveFromParent` (`self.UI`))))))
      (else
        (`Widget.RemoveFromParent` (`self.UI`))
        (`/Engine/EditorBlueprintResources/StandardMacros.IncrementInt` (`self.TalkIndex`)
          (:`  `
            (if (< (`self.TalkIndex`) (`KismetArrayLibrary.Array_Length` (`self.DialogueQuest1NotComplete`)))
              (bind _returnvalue_2 (`|CreateWidget` "/Game/NPC/Dialogue_WB.Dialogue_WB_C" (`GameplayStatics.GetPlayerController` 0)))
              (bind _output_get_2 (set `self.UI` _returnvalue_2))
              (`UserWidget.AddToViewport` _output_get_2 0)
              ;[1 1 1] Play Dialogue if Quest Not Complete
              (`TextBlock.SetText` (`/Game/NPC/Dialogue_WB.TalkText` (`self.UI`)) (`KismetTextLibrary.Conv_StringToText` (`|GetArrayItem` (`self.DialogueQuest1NotComplete`) (`self.TalkIndex`))))
              (`GameplayStatics.PlaySound2D` "/Game/MilitaryWeapSilver/Sound/Knife/Wavs/Knife_ImpactSurface03.Knife_ImpactSurface03" 1.0 1.0 0.0 null null)
              (else
                (set `self.TalkIndex` -1)
                (`Widget.RemoveFromParent` (`self.UI`))))))))
    (else
      (`/Engine/EditorBlueprintResources/StandardMacros.IncrementInt` (`self.TalkIndex`)
        (:`  `
          (if (< (`self.TalkIndex`) (`KismetArrayLibrary.Array_Length` (`self.DialogueQuest1Start`)))
            (`self.UI`
              (:`then`
                _)
              (:`else`
                (bind _returnvalue_3 (`|CreateWidget` "/Game/NPC/Dialogue_WB.Dialogue_WB_C" (`GameplayStatics.GetPlayerController` 0)))
                (bind _output_get_3 (set `self.UI` _returnvalue_3))
                (`UserWidget.AddToViewport` _output_get_3 0)))
            ;[1 1 1] Play Quest Start Dialogue
            (`TextBlock.SetText` (`/Game/NPC/Dialogue_WB.TalkText` (`self.UI`)) (`KismetTextLibrary.Conv_StringToText` (`|GetArrayItem` (`self.DialogueQuest1Start`) (`self.TalkIndex`))))
            (`GameplayStatics.PlaySound2D` "/Game/MilitaryWeapSilver/Sound/Knife/Wavs/Knife_ImpactSurface03.Knife_ImpactSurface03" 1.0 1.0 0.0 null null)
            (if (>= (`self.TalkIndex`) 2)
              (set `self.Quest1Start` true)
              (set `self.NewQuest` "Collect the Macguffin."))
            (else
              (set `self.TalkIndex` -1)
              (`Widget.RemoveFromParent` (`self.UI`)))))))))

(fn `UserConstructionScript`)